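; Lift Blueprint that moves between two points when the player character enters or leaves its Box trigger.
; Overlap begin and end each wait through a Delay, then play or reverse the Movement timeline.
; Each timeline update sets the Box's world location by lerping between the Move1 and Move2 positions, without sweep.
; A trailing Delay on the update has nothing wired after it.
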(event OnComponentBeginOverlap(Box)
  (params (OverlappedComponent :type Primitive%20Component%20Object%20Reference) (OtherActor :type Actor%20Object%20Reference) (OtherComp :type Primitive%20Component%20Object%20Reference) (OtherBodyIndex :type Integer) (bFromSweep :type Boolean) (SweepResult :type Hit%20Result%20Structure%20%28by%20ref%29))
  (if (== OtherActor (Game|GetPlayerCharacter 0))
    (Utilities|FlowControl|Delay 3.0)
    (CallFunction|ElevatorMoveUp)))

(event OnComponentEndOverlap(Box)
  (params (OverlappedComponent :type Primitive%20Component%20Object%20Reference) (OtherActor :type Actor%20Object%20Reference) (OtherComp :type Primitive%20Component%20Object%20Reference) (OtherBodyIndex :type Integer))
  (if (== OtherActor (Game|GetPlayerCharacter 0))
    (Utilities|FlowControl|Delay 3.0)
    (CallFunction|ElevatorMoveDown)))

(event Custom|Elevator%20Move%20Up
  (bind _0_to_1 (Timeline|Movement Play)
    (:Update
      (Transformation|SetWorldLocation (Variables|Default|GetBox) (Math|Vector|Lerp(Vector) (Transformation|GetWorldLocation (Variables|Default|GetMove1)) (Transformation|GetWorldLocation (Variables|Default|GetMove2)) _0_to_1) false false)
      (Utilities|FlowControl|Delay 3.0))))

(event Custom|Elevator%20Move%20down
  (bind _0_to_1 (Timeline|Movement Reverse)
    (:Update
      (Transformation|SetWorldLocation (Variables|Default|GetBox) (Math|Vector|Lerp(Vector) (Transformation|GetWorldLocation (Variables|Default|GetMove1)) (Transformation|GetWorldLocation (Variables|Default|GetMove2)) _0_to_1) false false)
      (Utilities|FlowControl|Delay 3.0))))

(fn ConstructionScript)