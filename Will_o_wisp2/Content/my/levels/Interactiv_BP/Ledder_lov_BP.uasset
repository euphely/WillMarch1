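; Interactive level Blueprint, apparently a ladder catch or lever, that triggers a one-time rotation when the player overlaps its Box.
; On overlap, if the Stop flag is set, it hides the MRuchRub mesh and reveals MRuchRub1 in its place.
; A timeline then drives the roll of the Center component, clearing Stop on each update so the trigger does not fire again.
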(event OnComponentBeginOverlap(Box)
  (params (OverlappedComponent :type Primitive%20Component%20Object%20Reference) (OtherActor :type Actor%20Object%20Reference) (OtherComp :type Primitive%20Component%20Object%20Reference) (OtherBodyIndex :type Integer) (bFromSweep :type Boolean) (SweepResult :type Hit%20Result%20Structure%20%28by%20ref%29))
  (if (== OtherActor (Game|GetPlayerCharacter 0))
    (if (Variables|Default|Getstop)
      (Development|SetHiddeninGame (Variables|Default|GetM_ruch_rub) true false)
      (Development|SetHiddeninGame (Variables|Default|GetM_ruch_rub1) false false)
      (bind _povorot (Timeline|Timeline_OneRotat Play)
        (:Update
          (Transformation|SetRelativeRotation (Variables|Default|Getcenter) (Math|Rotator|MakeRotator _povorot 0.0 0.0) false false)
          (Variables|Default|Setstop false))))))

(fn ConstructionScript)