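; Player character with an orthographic camera, built on the CustomMovement example, that loads doors_lvl when AngreMonster runs out.
; Inputs drive BP_CustomMovementComponent during custom movement, otherwise walking, jumping or FlyStart/FlyStop's small flying spirit form.
; Overlaps register mini_duh spirits, open History books and destroy spiders in monster form, while input triggers Les actors and zoom.
; A retry timer creates the health HUD; many spirit, stomp and transformation chains are disconnected.
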(event OnComponentBeginOverlap(CapsuleComponent)
  (params (OverlappedComponent :type Primitive%20Component%20Object%20Reference) (OtherActor :type Actor%20Object%20Reference) (OtherComp :type Primitive%20Component%20Object%20Reference) (OtherBodyIndex :type Integer) (bFromSweep :type Boolean) (SweepResult :type Hit%20Result%20Structure%20%28by%20ref%29))
  (if (== (Utilities|GetClass OtherActor) "/Game/my/menu/wi/history.history_C")
    (bind _returnvalue (UserInterface|CreateWidget "/Game/my/menu/wi/book.book_C"))
    (bind _output_get (Variables|Default|Setbook _returnvalue))
    (UserInterface|Viewport|AddtoViewport _output_get 0)
    (Variables|Default|Setbook_his (+ (Variables|Default|Getbook_his) 1.0))
    (Utilities|FlowControl|Delay 8.0)
    (if (not (Variables|/Script/Engine.PlayerController|GetbShowMouseCursor (Game|GetPlayerController 0)))
      (bind _returnvalue_2 (UserInterface|CreateWidget "/Game/Widgets/WD_LiquidHealth.WD_LiquidHealth_C"))
      (bind _output_get_2 (Variables|Default|Sethud_test_inTwo_0 _returnvalue_2))
      (UserInterface|Viewport|AddtoViewport _output_get_2 0))))

(event OnComponentBeginOverlap(Top_box)
  (params (OverlappedComponent :type Primitive%20Component%20Object%20Reference) (OtherActor :type Actor%20Object%20Reference) (OtherComp :type Primitive%20Component%20Object%20Reference) (OtherBodyIndex :type Integer) (bFromSweep :type Boolean) (SweepResult :type Hit%20Result%20Structure%20%28by%20ref%29))
  (if (Variables|Default|GetMonster_form)
    (if (== (Utilities|GetClass OtherActor) "/Game/Ai/spider_body_SideScrollerCharacter1.spider_body_SideScrollerCharacter1_C")
      (if (Variables|Default|GetTop_tru)
        (bind _asspider_body_side_scroller_character_1 (Utilities|Casting|CastTospider_body_SideScrollerCharacter1 OtherActor))
        (Actor|DestroyActor _asspider_body_side_scroller_character_1)))))

(event OnStartCustomMovement(BP_CustomMovementComponent)
  ;[1 1 1] The OnStartCustomMovement event dispatcher of BP_CustomMovementComponent is called when the character starts CustomMovement.
)

(event OnEndCustomMovement(BP_CustomMovementComponent)
  ;[1 1 1] The OnEndCustomMovement event dispatcher of BP_CustomMovementComponent is called when the character ends CustomMovement.
)

(event Custom|create%20hp%20widget
  ;[1 1 1] hud_monitor
  (if (Variables|Default|Getstope_widget)
    (Variables|Default|Setwidget%20ok true)
    (bind _foundwidgets (Widget|GetAllWidgetsOfClass "/Script/UMG.UserWidget" true))
    (for _array_element _foundwidgets
      (if (Widget|IsVisible _array_element)
        (Variables|Default|Setwidget%20ok false)
        (bind _returnvalue (UserInterface|CreateWidget "/Game/Widgets/WD_LiquidHealth.WD_LiquidHealth_C"))
        (bind _output_get (Variables|Default|Sethud_test_inTwo_0 _returnvalue))
        (UserInterface|Viewport|AddtoViewport _output_get 0)
        (Variables|Default|Setstope_widget false)))
    (if (Variables|Default|Getwidget%20ok)
      (bind _returnvalue_2 (UserInterface|CreateWidget "/Game/Widgets/WD_LiquidHealth.WD_LiquidHealth_C"))
      (bind _output_get_2 (Variables|Default|Sethud_test_inTwo_0 _returnvalue_2))
      (UserInterface|Viewport|AddtoViewport _output_get_2 0)
      (Variables|Default|Setstope_widget false)
      (else
        (Utilities|Time|SetTimerbyEvent (delegate Custom|create%20hp%20widget) 1.0)))))

(event EventBeginPlay
  (Utilities|FlowControl|Sequence
    (:then_0
      (bind _outactors (Actor|GetAllActorsOfClass "/Game/my/sad/forest/les.les_C"))
      (Variables|Default|Setless (Math|Conversions|ToFloat(Integer) (Utilities|Array|Length _outactors))))
    (:then_1
      (Utilities|Time|SetTimerbyEvent (delegate Custom|create%20hp%20widget) 1.0))))

(event EventUpdateCustomMovement
  (params (DeltaTime :type Float%20%28single-precision%29))
  ;[1 1 1] UpdateCustomMovement
  ; CustomMovement uses the "Custom" Movement Mode of CharacterMovement.
  ; In your character's UpdateCustomMovement event, you need to call the UpdateCustomMovement event of BP_CustomMovementComponent.
  (Default|UpdateCustomMovement (Variables|Default|GetBP_CustomMovementComponent) DeltaTime))

(event EventTick
  (params (DeltaSeconds :type Float%20%28single-precision%29))
  (Utilities|FlowControl|Sequence
    (:then_0
      (if (<= (Variables|Default|GetAngreMonster) 0.0)
        (Game|OpenLevel(byName) "doors_lvl")))
    (:then_1
      (Transformation|SetWorldRotation (Variables|Default|GetMesto_L_for_bubl) "0,-90.000000,0.000000" false false))))

(event Collision|EventActorBeginOverlap
  (params (OtherActor :type Actor%20Object%20Reference))
  (Utilities|FlowControl|Sequence
    (:then_0
      (bind _asmini_duh (Utilities|Casting|CastTomini_duh OtherActor))
      (Utilities|Array|Add (Variables|Default|Getciplyta) _asmini_duh)
      (Variables|/Game/my/duh_mini/mini_duh.mini_duh_C|Setyou _asmini_duh self))
    (:then_1
      (bind _asfor_timer_w (Utilities|Casting|CastTofor_timer_w OtherActor))
      (Variables|Default|Setcast_timer_tutr _asfor_timer_w))))

(event Input|ActionEvents|InputActionDeystvie
  (params (Key :type Key%20Structure :default "None"))
  (:Pressed
    (for _array_element (Collision|GetOverlappingActors "/Game/my/sad/forest/les.les_C" :!class /Script/Engine.Actor)
      (bind _asles (Utilities|Casting|CastToles _array_element))
      (Default|DvigTrigerfromCharecter _asles))))

(event Input|ActionEvents|InputActionzoom
  (params (Key :type Key%20Structure :default "None"))
  (bind _returnvalue (Game|GetPlayerController 0))
  (:Pressed
    (Variables|/Script/Engine.PlayerController|SetbShowMouseCursor _returnvalue true))
  (:Released
    (Variables|/Script/Engine.PlayerController|SetbShowMouseCursor _returnvalue false)))

(event Input|ActionEvents|InputActionJump
  (params (Key :type Key%20Structure :default "None"))
  (:Pressed
    (if (not (Variables|Default|GetMonster_form))
      ;[1 1 1] Jump
      ; If the character is in CustomMovment, it will escape its CustomMovement.
      (Utilities|IsCustomMovement
        (:True
          (Default|ExitCustomMovement (Variables|Default|GetBP_CustomMovementComponent)))
        (:False
          (Character|Jump)))))
  (:Released
    (Character|StopJumping)))

(event Input|AxisEvents|InputAxismy_up_down
  (params (AxisValue :type Float%20%28single-precision%29))
  ;[1 1 1] Movement input
  ; Processes user input based on whether the character is a CustomMovment.
  (Utilities|IsCustomMovement
    (:True
      (Default|AddCustomMovementInputUp (Variables|Default|GetBP_CustomMovementComponent) AxisValue))
    (:False
      (if (Variables|Default|Getfly_trub)
        (Pawn|Input|AddMovementInput "0, 0,1.000000" AxisValue false)))))

(event Input|AxisEvents|InputAxisfly_trub
  (params (AxisValue :type Float%20%28single-precision%29)))

(event Input|AxisEvents|InputAxiszoom_p
  (params (AxisValue :type Float%20%28single-precision%29))
  (bind _camera (Variables|Default|GetCamera))
  (bind _orthowidth (Variables|/Script/Engine.CameraComponent|GetOrthoWidth _camera))
  (bind _returnvalue (+ _orthowidth 25.0))
  (if (Variables|/Script/Engine.PlayerController|GetbShowMouseCursor (Game|GetPlayerController 0))
    (Development|PrintString (Utilities|String|ToString(Float) _returnvalue))
    (Class|CameraComponent|SetOrthoWidth _camera _returnvalue)))

(event Input|AxisEvents|InputAxisMoveRight
  (params (AxisValue :type Float%20%28single-precision%29))
  ;[1 1 1] Movement input
  ; Processes user input based on whether the character is a CustomMovment.
  (Utilities|IsCustomMovement
    (:True
      (Default|AddCustomMovementInputRight (Variables|Default|GetBP_CustomMovementComponent) AxisValue))
    (:False
      (Pawn|Input|AddMovementInput "0.000000,-1.000000,0.000000" AxisValue false))))

(event Input|KeyboardEvents|R
  (params (Key :type Key%20Structure :default "None")))

(fn ConstructionScript)

(fn FlyStart
  (Variables|Default|Setfly_trub true)
  (Pawn|Components|CharacterMovement|SetMovementMode (Variables|Character|GetCharacterMovement) "MOVE_Flying" 0)
  (Development|SetHiddeninGame (Variables|Character|GetMesh) true false)
  (Development|SetHiddeninGame (Variables|Default|Getduh_form) false false)
  (Development|SetHiddeninGame (Variables|Default|Getfi_rere) false false)
  (Transformation|SetRelativeScale3D (Variables|Transformation|GetRootComponent) "0.300000,0.300000,0.300000")
  (for _array_element (Actor|GetAttachedActors true)
    (Rendering|SetActorHiddenInGame _array_element true)))

(fn FlyStop
  (Variables|Default|Setfly_trub false)
  (Pawn|Components|CharacterMovement|SetMovementMode (Variables|Character|GetCharacterMovement) "MOVE_Walking" 0)
  (Development|SetHiddeninGame (Variables|Character|GetMesh) false false)
  (Development|SetHiddeninGame (Variables|Default|Getduh_form) true false)
  (Development|SetHiddeninGame (Variables|Default|Getfi_rere) true false)
  (Transformation|SetRelativeScale3D (Variables|Transformation|GetRootComponent) "1.000000,1.000000,1.000000")
  (for _array_element (Actor|GetAttachedActors true)
    (Rendering|SetActorHiddenInGame _array_element true)))

(fn NewFunction0)

(fn Interactiv)

(fn Zoom)

(fn CanEnteringCustomMovement
  (params (CustomMoveZone :type S%20Custom%20Move%20Zone%20Structure) (ImmediateEntryRequired :type Boolean))
  ;[1 1 1] This function determines whether a character can start CustomMovement.
  ; If the value of ImmediateEntryRequired is true, the wait time will be ignored on entry.
  (return true))

(fn GetCustomMovement
  ;[1 1 1] This function returns the character's BP_CustomMovementComponent.
  (return (Variables|Default|GetBP_CustomMovementComponent)))

(fn OnBeforeStartCustomMovement
  (params (CustomMoveZone :type S%20Custom%20Move%20Zone%20Structure))
  ;[1 1 1] This function is called before the character starts CustomMovement.
  ; From here, you can handle prior tasks such as hiding weapons or changing posture.
  ; If you need time to proceed with the preceding task, you can return the time to delay the start of CustomMovement.
  (return 0.0))